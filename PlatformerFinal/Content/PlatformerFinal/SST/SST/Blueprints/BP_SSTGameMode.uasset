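; BP_SSTGameMode is a game mode that keeps an elapsed-time count in minutes and seconds.
; StartTimer sets a looping 0.01-second timer bound to itself, so each tick re-sets that timer and advances TimerSeconds.
; TimerMinutes increments on every tick where seconds are at least 60, with no seconds reset in this graph.
; StopTimer pauses the count through the stored timer handle.
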(event Custom|Start%20Timer
  (bind _returnvalue (Utilities|Time|SetTimerbyEvent (delegate Custom|Start%20Timer) 0.01 true))
  (Variables|Default|SettimerSeconds (+ (Variables|Default|GettimerSeconds) 0.01))
  (if (>= (Variables|Default|GettimerSeconds) 6e+01)
    (Variables|Default|SettimerMinutes (+ (Variables|Default|GettimerMinutes) 1.0))))

(event Custom|Stop%20Timer
  (Utilities|Time|PauseTimerbyHandle (stale Custom|Start%20Timer _returnvalue)))

(fn ConstructionScript)